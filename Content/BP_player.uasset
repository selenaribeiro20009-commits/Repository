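; Player Blueprint that moves a Cube component with physics impulses from WASD and Space bar input.
; Key press and release events toggle movement and jump flags, which Tick checks each frame to add velocity-change impulses along fixed world axes.
; Impulses are not scaled by delta time, and jump has no ground check, so holding Space keeps pushing the cube upward.
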(event EventBeginPlay
  (Development|PrintString "Hello"))

(event EventTick
  (params (DeltaSeconds :type Float%20%28single-precision%29))
  (Utilities|FlowControl|Sequence
    (:then_0
      (if (Variables|Default|GetMove%20Forward)
        (Physics|AddImpulse (Variables|Default|GetCube) "10.000000,0.000000,0.000000" "None" true)))
    (:then_1
      (if (Variables|Default|GetMove%20Backward)
        (Physics|AddImpulse (Variables|Default|GetCube) "-10.000000,0.000000,0.000000" "None" true)))
    (:then_2
      (if (Variables|Default|GetMove%20Right)
        (Physics|AddImpulse (Variables|Default|GetCube) "0.000000,10.000000,0.000000" "None" true)))
    (:then_3
      (if (Variables|Default|GetMove%20Left)
        (Physics|AddImpulse (Variables|Default|GetCube) "0.000000,-10.000000,0.000000" "None" true)))
    (:then_4
      (if (Variables|Default|GetJump)
        (Physics|AddImpulse (Variables|Default|GetCube) "0.000000,0.000000,30.000000" "None" true)))))

(event Input|KeyboardEvents|W
  (params (Key :type Key%20Structure :default "None"))
  (:Pressed
    (Variables|Default|SetMove%20Forward true))
  (:Released
    (Variables|Default|SetMove%20Forward false)))

(event Input|KeyboardEvents|S
  (params (Key :type Key%20Structure :default "None"))
  (:Pressed
    (Variables|Default|SetMove%20Backward true))
  (:Released
    (Variables|Default|SetMove%20Backward false)))

(event Input|KeyboardEvents|D
  (params (Key :type Key%20Structure :default "None"))
  (:Pressed
    (Variables|Default|SetMove%20Right true))
  (:Released
    (Variables|Default|SetMove%20Right false)))

(event Input|KeyboardEvents|A
  (params (Key :type Key%20Structure :default "None"))
  (:Pressed
    (Variables|Default|SetMove%20Left true))
  (:Released
    (Variables|Default|SetMove%20Left false)))

(event Input|KeyboardEvents|SpaceBar
  (params (Key :type Key%20Structure :default "None"))
  (:Pressed
    (Variables|Default|SetJump true))
  (:Released
    (Variables|Default|SetJump false)))

(fn ConstructionScript)